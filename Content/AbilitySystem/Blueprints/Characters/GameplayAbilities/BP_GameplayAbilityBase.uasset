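; Base Gameplay Ability Blueprint that supplies shared helpers for character abilities, with no activation logic of its own.
; A helper resolves the owning BP_CharacterBase and its BP_PlayerController for the other functions.
; DoUICooldown starts the cooldown on primary UI slots whose ability class matches this ability's info.
; IsCostStillAvailable negates the ability cost and checks that the character's Health, Mana or Strength, chosen by cost type, exceeds it.
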(fn `DoUICooldown`
  (bind (_characterbase _playercontrollerbase) (`self.Get Player Character and Controller`))
  (`/Engine/EditorBlueprintResources/StandardMacros.IsValid` _playercontrollerbase
    (:`Is Valid`
      (for _array_element (`/Game/AbilitySystem/UI/WBP_PrimaryUI.Slots` (`/Game/AbilitySystem/Blueprints/BP_PlayerController.PrimaryUI` _playercontrollerbase))
        (bind _returnvalue (`self.GetAbilityInfo`))
        (bind (_abilityinfo_cooldownduration _abilityinfo_cost _abilityinfo_costtype _abilityinfo_uimat _abilityinfo_abilityclass) (break `GameplayAbilityInfo` (`/Game/AbilitySystem/UI/WBP_Ability_Slot.AbilityInfo` _array_element)))
        (if (== (`.AbilityClass` (break `GameplayAbilityInfo` _returnvalue)) _abilityinfo_abilityclass)
          (`/Game/AbilitySystem/UI/WBP_Ability_Slot.StartCoolDown` _array_element))))))

(fn `Get Player Character and Controller`
  (returns (CharacterBase :type "/Game/AbilitySystem/Blueprints/Characters/BP_CharacterBase Object Reference") (PlayerControllerBase :type "/Game/AbilitySystem/Blueprints/BP_PlayerController Object Reference"))
  (bind _asbp_character_base (cast `/Game/AbilitySystem/Blueprints/Characters/BP_CharacterBase` (`self.GetOwningActorFromActorInfo`))
    (:`then`
      (bind _asbp_player_controller (cast `/Game/AbilitySystem/Blueprints/BP_PlayerController` (`Pawn.GetController` _asbp_character_base))
        (:`then`
          _)
        (:`CastFailed`
          _)))
    (:`CastFailed`
      _))
  (return _asbp_character_base _asbp_player_controller))

(fn `IsCostStillAvailable`
  (returns (Can :type Boolean))
  (locals (Cost :type "Float (double-precision)"))
  (bind _returnvalue (`self.GetAbilityInfo`))
  (set `local.Cost` (* (`.Cost` (break `GameplayAbilityInfo` _returnvalue)) -1.0))
  (switch `EAbilityCostType` (`.CostType` (break `GameplayAbilityInfo` _returnvalue))
    (:`Health`
      ;[1 0.66 0.66] Can Spend Health?
      (bind _characterbase (`self.Get Player Character and Controller`))
      (bind (_health_basevalue _health_currentvalue) (break `GameplayAttributeData` (`AttributeSetBase.Health` (`CharacterBase.AttributeSetBaseComp` _characterbase))))
      (return (> _health_currentvalue (`local.Cost`))))
    (:`Mana`
      ;[0.66 0.66 1] Can Spend Mana?
      (bind _characterbase_2 (`self.Get Player Character and Controller`))
      (bind (_mana_basevalue _mana_currentvalue) (break `GameplayAttributeData` (`AttributeSetBase.Mana` (`CharacterBase.AttributeSetBaseComp` _characterbase_2))))
      (return (> _mana_currentvalue (`local.Cost`))))
    (:`Strength`
      ;[0.66 1 0.66] Can Spend Strength?
      (bind _characterbase_3 (`self.Get Player Character and Controller`))
      (bind (_strength_basevalue _strength_currentvalue) (break `GameplayAttributeData` (`AttributeSetBase.Strength` (`CharacterBase.AttributeSetBaseComp` _characterbase_3))))
      (return (> _strength_currentvalue (`local.Cost`))))))