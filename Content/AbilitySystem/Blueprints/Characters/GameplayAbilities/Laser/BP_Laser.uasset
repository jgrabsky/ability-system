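; Laser beam actor that periodically signals damage for hostile characters touching its end detector, as part of a Gameplay Ability System skill.
; Tick feeds the detector's distance, relative to the original beam length, into the anim blueprint's end bone offset to stretch the mesh.
; Detector overlaps maintain a list of characters hostile to the instigator.
; A looping timer sends that list to the instigator as target data in a gameplay event.
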(event `self.ReceiveBeginPlay`
  (set `self.BeamOriginalLength` (`KismetMathLibrary.VSize` (- (`SceneComponent.GetSocketLocation` (`self.LaserMesh`) "End") (`self.K2_GetActorLocation`))))
  ;[1 0.3 0.3] Send Laser Damage Event per 0.3 Seconds
  (`KismetSystemLibrary.K2_SetTimerDelegate` (delegate `SendDealDamage`) 0.3 true))

(event `SendDealDamage`
  (bind _overlappingactors (`self.OverlappingActors`))
  ;[1 0.3 0.3] Send Laser Damage Event per 0.3 Seconds
  (if (`KismetMathLibrary.Conv_IntToBool` (`KismetArrayLibrary.Array_Length` _overlappingactors))
    _
    (else
      _))
  (`AbilitySystemBlueprintLibrary.SendGameplayEventToActor` (`self.GetInstigator`) (struct :`TagName` "skill.laser.dealDamage") (make `GameplayEventData` (struct) null null null null (struct) (struct) (struct) 0.0 (`AbilitySystemBlueprintLibrary.AbilityTargetDataFromActorArray` _overlappingactors))))

(event `self.ReceiveTick`
  (params (DeltaSeconds :type "Float (single-precision)"))
  (bind _asanim_bp_laser_beam (cast `/Game/AbilitySystem/Blueprints/Characters/GameplayAbilities/Laser/LaserAssets/AnimBP_LaserBeam` (`SkeletalMeshComponent.GetAnimInstance` (`self.LaserMesh`))))
  (set `/Game/AbilitySystem/Blueprints/Characters/GameplayAbilities/Laser/LaserAssets/AnimBP_LaserBeam.EndBoneOffset` (`KismetMathLibrary.MakeVector` (- (`KismetMathLibrary.VSize` (- (`SceneComponent.K2_GetComponentLocation` (`self.LaserEndDetector`)) (`self.K2_GetActorLocation`))) (`self.BeamOriginalLength`))) _asanim_bp_laser_beam))

(event `self.LaserEndDetector.OnComponentBeginOverlap`
  (params (OverlappedComponent :type "PrimitiveComponent Object Reference") (OtherActor :type "Actor Object Reference") (OtherComp :type "PrimitiveComponent Object Reference") (OtherBodyIndex :type Integer) (bFromSweep :type Boolean) (SweepResult :type "HitResult Structure (by ref)"))
  (bind _asbp_character_base (cast `/Game/AbilitySystem/Blueprints/Characters/BP_CharacterBase` OtherActor))
  (bind _asbp_character_base_2 (cast `/Game/AbilitySystem/Blueprints/Characters/BP_CharacterBase` (`self.GetInstigator`)))
  (bind _returnvalue (`CharacterBase.IsOtherHostile` _asbp_character_base_2 _asbp_character_base))
  (if _returnvalue
    (`KismetArrayLibrary.Array_AddUnique` (`self.OverlappingActors`) _asbp_character_base)))

(event `self.LaserEndDetector.OnComponentEndOverlap`
  (params (OverlappedComponent :type "PrimitiveComponent Object Reference") (OtherActor :type "Actor Object Reference") (OtherComp :type "PrimitiveComponent Object Reference") (OtherBodyIndex :type Integer))
  (bind _asbp_character_base (cast `/Game/AbilitySystem/Blueprints/Characters/BP_CharacterBase` OtherActor))
  (`KismetArrayLibrary.Array_RemoveItem` (`self.OverlappingActors`) _asbp_character_base))

(fn `UserConstructionScript`)