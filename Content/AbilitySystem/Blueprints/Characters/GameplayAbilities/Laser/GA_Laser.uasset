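; Laser gameplay ability that plays a casting montage, then after a short delay spawns BP_Laser on the character's mesh "laser" socket and enables camera-control rotation.
; Each deal-damage gameplay event applies laser damage to its targets and pushes hit characters away from the beam's end with a stun, ending the ability when cost runs out.
; On end, it removes the cost-drain effect, destroys the laser and again passes true to camera-control rotation.
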(event `self.K2_ActivateAbility`
  (`parent.K2_ActivateAbility`)
  (`self.K2_CommitAbility`)
  (`self.DoUICooldown`)
  (`AbilityTask_PlayMontageAndWait.CreatePlayMontageAndWaitProxy` "None" "/Game/AbilitySystem/Blueprints/Characters/Animation/AM_Laser_Casting.AM_Laser_Casting"
    (:`then`
      (`KismetSystemLibrary.Delay` 0.3)
      (bind _characterbase (`self.Get Player Character and Controller`))
      (bind (_asynctaskproxy _spawnedactor) (`AbilityTask_SpawnActor.SpawnActor` (struct) "/Game/AbilitySystem/Blueprints/Characters/GameplayAbilities/Laser/BP_Laser.BP_Laser_C" _characterbase)
        (:`then`
          (bind _output_get (set `self.LaserActor` _spawnedactor))
          (`Actor.K2_AttachToComponent` _output_get (`Character.Mesh` _characterbase) "laser" "SnapToTarget" "SnapToTarget" "KeepRelative" true)
          (`/Game/AbilitySystem/Blueprints/Characters/BP_CharacterBase.MakeCameraControlRotation` _characterbase true)
          (bind (_asynctaskproxy_2 _payload) (`AbilityTask_WaitGameplayEvent.WaitGameplayEvent` (struct :`TagName` "skill.laser.dealDamage") null)
            (:`EventReceived`
              (bind _can (`self.IsCostStillAvailable`))
              (if _can
                (bind (_eventtag _instigator _target _optionalobject _optionalobject2 _contexthandle _instigatortags _targettags _eventmagnitude _targetdata) (break `GameplayEventData` _payload))
                (`self.BP_ApplyGameplayEffectToTarget` _targetdata "/Game/AbilitySystem/Blueprints/Characters/GameplayAbilities/Laser/GE_Laser_Damage.GE_Laser_Damage_C")
                (for _array_element (`AbilitySystemBlueprintLibrary.GetActorsFromTargetData` _targetdata)
                  (bind _asbp_character_base (cast `/Game/AbilitySystem/Blueprints/Characters/BP_CharacterBase` _array_element))
                  (`/Game/AbilitySystem/Blueprints/Characters/BP_CharacterBase.Push Character` _asbp_character_base (`KismetMathLibrary.Normal` (- (`Actor.K2_GetActorLocation` _asbp_character_base) (`SceneComponent.K2_GetComponentLocation` (`/Game/AbilitySystem/Blueprints/Characters/GameplayAbilities/Laser/BP_Laser.LaserEndDetector` (cast `/Game/AbilitySystem/Blueprints/Characters/GameplayAbilities/Laser/BP_Laser` (`self.LaserActor`) :!pure true))))) 500.0 0.3 "/Game/AbilitySystem/Blueprints/Characters/Animation/AM_HitStun_Shinbi.AM_HitStun_Shinbi"))
                (else
                  (`self.K2_EndAbility`))))))))))

(event `self.K2_OnEndAbility`
  (params (bWasCancelled :type Boolean))
  (`parent.K2_OnEndAbility` bWasCancelled)
  (`self.BP_RemoveGameplayEffectFromOwnerWithAssetTags` (struct :`GameplayTags` (struct :`(TagName` "skill.laser.drainCost"))))
  (`Actor.K2_DestroyActor` (`self.LaserActor`))
  (bind _characterbase (`self.Get Player Character and Controller`))
  (`/Game/AbilitySystem/Blueprints/Characters/BP_CharacterBase.MakeCameraControlRotation` _characterbase true))