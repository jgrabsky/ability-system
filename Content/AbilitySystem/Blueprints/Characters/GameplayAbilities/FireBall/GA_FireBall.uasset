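; GA_FireBall is a gameplay ability that launches a fireball after a casting animation.
; On activation it commits, runs the UI cooldown and plays a Shinbi melee combo montage.
; Montage completion spawns BP_FireBall at the player character's transform, passing it the instigator and a GE_Dash_Damage effect spec, then ends the ability.
; Blend out, interruption or cancellation ends the ability without spawning.
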(event `self.K2_ActivateAbility`
  (`parent.K2_ActivateAbility`)
  (`self.K2_CommitAbility`)
  (`self.DoUICooldown`)
  (`AbilityTask_PlayMontageAndWait.CreatePlayMontageAndWaitProxy` "None" "/Game/AbilitySystem/Blueprints/Characters/Animation/AM_Shinbi_Melee_Combo_03.AM_Shinbi_Melee_Combo_03"
    (:`OnCompleted`
      (bind _characterbase (`self.Get Player Character and Controller`))
      (`|SpawnActorFromClass` "/Game/AbilitySystem/Blueprints/Characters/GameplayAbilities/FireBall/BP_FireBall.BP_FireBall_C" (`Actor.GetTransform` _characterbase) "AlwaysSpawn" "OverrideRootScale" null (`self.MakeOutgoingGameplayEffectSpec` "/Game/AbilitySystem/Blueprints/Characters/GameplayAbilities/Dash/GE_Dash_Damage.GE_Dash_Damage_C") _characterbase)
      (`self.K2_EndAbility`))
    (:`OnBlendOut`
      (`self.K2_EndAbility` :!label _label))
    (:`OnInterrupted`
      (goto _label))
    (:`OnCancelled`
      (goto _label))))