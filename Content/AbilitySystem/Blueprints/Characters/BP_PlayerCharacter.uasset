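; Player character Blueprint that mirrors its health, mana and strength on the player's HUD.
; Attribute change events cast the controller to BP_PlayerController and pass the current-to-max ratio to the matching glass ball widget in its PrimaryUI.
; The graph is purely event-driven: Tick and BeginPlay are disabled stubs, and the construction script only calls its parent.
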(event `self.BP_OnHealthChanged`
  (params (Health :type "Float (single-precision)") (MaxHealth :type "Float (single-precision)"))
  (bind _asbp_player_controller (cast `/Game/AbilitySystem/Blueprints/BP_PlayerController` (`self.GetController`)))
  (`/Game/AbilitySystem/UI/WBP_GlassBall.SetPercentage` (`/Game/AbilitySystem/UI/WBP_PrimaryUI.WBP_HealthGlassBall` (`/Game/AbilitySystem/Blueprints/BP_PlayerController.PrimaryUI` _asbp_player_controller)) (/ Health MaxHealth)))

(event `self.BP_OnManaChanged`
  (params (Mana :type "Float (single-precision)") (MaxMana :type "Float (single-precision)"))
  (bind _asbp_player_controller (cast `/Game/AbilitySystem/Blueprints/BP_PlayerController` (`self.GetController`)))
  (`/Game/AbilitySystem/UI/WBP_GlassBall.SetPercentage` (`/Game/AbilitySystem/UI/WBP_PrimaryUI.WBP_ManaGlassBall` (`/Game/AbilitySystem/Blueprints/BP_PlayerController.PrimaryUI` _asbp_player_controller)) (/ Mana MaxMana)))

(event `self.BP_OnStrengthChanged`
  (params (Strength :type "Float (single-precision)") (MaxStrength :type "Float (single-precision)"))
  (bind _asbp_player_controller (cast `/Game/AbilitySystem/Blueprints/BP_PlayerController` (`self.GetController`)))
  (`/Game/AbilitySystem/UI/WBP_GlassBall.SetPercentage` (`/Game/AbilitySystem/UI/WBP_PrimaryUI.WBP_StrengthGlassBall` (`/Game/AbilitySystem/Blueprints/BP_PlayerController.PrimaryUI` _asbp_player_controller)) (/ Strength MaxStrength)))

(fn `UserConstructionScript`
  (`parent.UserConstructionScript`))